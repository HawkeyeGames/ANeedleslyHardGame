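; BP_PitTrapTrigger is a trap actor that kills the side-scroller player on contact and restarts the level.
; On overlap with BP_SideScrollerCharacter, it blocks the player's move input, removes the PitMesh collision and destroys that mesh so the floor gives way.
; It then sets the character's Dead flag, waits briefly and reloads the current level by name.
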(event `self.ReceiveActorBeginOverlap`
  (params (OtherActor :type "Actor Object Reference"))
  (bind _pitmesh (`self.PitMesh`))
  (bind _asbp_side_scroller_character (cast `/Game/SideScrollerCPP/Blueprints/BP_SideScrollerCharacter` OtherActor))
  (`Controller.SetIgnoreMoveInput` (`GameplayStatics.GetPlayerController` 0) true)
  (`PrimitiveComponent.SetCollisionEnabled` _pitmesh "NoCollision")
  (`ActorComponent.K2_DestroyComponent` _pitmesh)
  (set `ANeedleslyHardGameCharacter.bDead` true _asbp_side_scroller_character)
  (`KismetSystemLibrary.Delay` 0.5)
  (bind _returnvalue (`GameplayStatics.GetCurrentLevelName` true))
  (`GameplayStatics.OpenLevel` (`KismetStringLibrary.Conv_StringToName` _returnvalue)))

(fn `UserConstructionScript`)