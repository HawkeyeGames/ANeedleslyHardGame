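; Turret trap that kills the run when the side-scroller character enters its trigger box, by firing and then reloading the current level.
; If CanTrigger is set, the overlap runs a one-shot timed sequence: slide the neck to EndLocation, call Shoot with sound cues, then reopen the level.
; Once triggered, Tick blinks the gun's red light by flip-flopping its material through a Delay.
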(event `self.ReceiveTick`
  (params (DeltaSeconds :type "Float (single-precision)"))
  (bind _gun (`self.Gun`))
  (if (`self.bTriggered`)
    (`KismetSystemLibrary.Delay` 0.5)
    (`/Engine/EditorBlueprintResources/StandardMacros.FlipFlop`
      (:`A`
        (`PrimitiveComponent.SetMaterial` _gun 2 "/Game/Objects/Traps/Meshes/Materials/Red_Light_Inst.Red_Light_Inst"))
      (:`B`
        (`PrimitiveComponent.SetMaterial` _gun 2 "/Game/Objects/Traps/Meshes/Materials/Red_Light_Off_Inst.Red_Light_Off_Inst")))))

(event `self.TriggerBox.OnComponentBeginOverlap`
  (params (OverlappedComponent :type "PrimitiveComponent Object Reference") (OtherActor :type "Actor Object Reference") (OtherComp :type "PrimitiveComponent Object Reference") (OtherBodyIndex :type Integer) (bFromSweep :type Boolean) (SweepResult :type "HitResult Structure (by ref)"))
  (cast `/Game/SideScrollerCPP/Blueprints/BP_SideScrollerCharacter` OtherActor)
  (if (`self.bCanTrigger`)
    (`/Engine/EditorBlueprintResources/StandardMacros.DoOnce` false
      (:`Completed`
        (set `self.bTriggered` true)
        (`GameplayStatics.PlaySound2D` "/Game/Sounds/SFX/Turret/gun_mid_air.gun_mid_air" 1.0 1.0 0.0 null null)
        (`KismetSystemLibrary.MoveComponentTo` (`self.Neck`) (`self.EndLocation`) (struct) true true 1.0)
        (`KismetSystemLibrary.Delay` 2.0)
        (`GameplayStatics.PlaySound2D` "/Game/Sounds/SFX/Turret/gun_shoot.gun_shoot" 1.0 1.0 0.0 null null)
        (`KismetSystemLibrary.Delay` 0.2)
        (`self.Shoot`)
        (`GameplayStatics.PlaySound2D` "/Game/Sounds/SFX/Turret/gun_hit.gun_hit" 1.0 1.0 0.0 null null)
        (`KismetSystemLibrary.Delay` 2.0)
        (bind _returnvalue (`GameplayStatics.GetCurrentLevelName` true))
        (`GameplayStatics.OpenLevel` (`KismetStringLibrary.Conv_StringToName` _returnvalue))))))

(fn `UserConstructionScript`)