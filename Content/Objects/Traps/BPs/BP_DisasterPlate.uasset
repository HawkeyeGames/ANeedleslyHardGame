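; BP_DisasterPlate is a trap plate whose TriggerDisaster event sends the side-scroller player back to PlayerStart.
; It flags every plate as triggered, moves its plate mesh, and disables player move input, jumping and gravity.
; A timeline lerps the character to the start while a delay later restores control and clears the flags.
; An unconnected earthquake sequence with camera shake, physics collapse and level reload never runs.
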(event `self.TriggerDisaster`
  (bind _outactors (`GameplayStatics.GetAllActorsOfClass` "BP_DisasterPlate_C"))
  (for _array_element _outactors
    (set `DisasterPlate.bTriggered` true _array_element)
    (set `self.bTriggered` true))
  (`KismetSystemLibrary.MoveComponentTo` (`self.Plate`) (0.0 0.0 1.0) (struct) true true)
  (`Controller.SetIgnoreMoveInput` (`GameplayStatics.GetPlayerController` 0) true)
  (bind _asbp_side_scroller_character (cast `/Game/SideScrollerCPP/Blueprints/BP_SideScrollerCharacter` (`GameplayStatics.GetPlayerCharacter` 0)))
  (set `ANeedleslyHardGameCharacter.bCanJump` false _asbp_side_scroller_character)
  (set `CharacterMovementComponent.GravityScale` 0.0 (`Character.CharacterMovement` _asbp_side_scroller_character))
  (`|ExecutionSequence`
    (:`then_0`
      (bind (_direction _alpha) (`Timeline|MovePlayer` :!via `PlayFromStart`)
        (:`Update`
          (`self.K2_SetActorLocation` _asbp_side_scroller_character (`KismetMathLibrary.VLerp` (`self.K2_GetActorLocation` _asbp_side_scroller_character) (`self.PlayerStart`) _alpha) false false))))
    (:`then_1`
      (`KismetSystemLibrary.Delay` 3.0)
      (`Controller.SetIgnoreMoveInput` (`GameplayStatics.GetPlayerController` 0) false)
      (set `ANeedleslyHardGameCharacter.bCanJump` true _asbp_side_scroller_character)
      (set `CharacterMovementComponent.GravityScale` 2.0 (`Character.CharacterMovement` _asbp_side_scroller_character))
      (bind _outactors_2 (`GameplayStatics.GetAllActorsOfClass` "BP_DisasterPlate_C"))
      (for _array_element_2 _outactors_2
        (set `DisasterPlate.bTriggered` false _array_element_2)
        (set `self.bTriggered` false)))))

(fn `UserConstructionScript`)